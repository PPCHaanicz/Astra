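; Enemy ship projectile that flies in a straight line along its MoveVector at its Speed and destroys itself after a fixed lifetime.
; BeginPlay attaches an energy ball Niagara effect to the Sphere component and starts the delayed destroy.
; Tick moves the actor manually with a swept, frame-rate-independent SetActorLocation.
; The graph has no hit or damage logic, as the overlap event is an empty, disabled stub.
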(event `self.ReceiveBeginPlay`
  (`NiagaraFunctionLibrary.SpawnSystemAttached` "/Game/Assets/EnergyBall/NS_EnergyBall.NS_EnergyBall" (`self.Sphere`) "None" (0.0 0.0 0.0) (struct :`Yaw` 90.0) "KeepRelativeOffset")
  (`KismetSystemLibrary.Delay` 5.0)
  (`self.K2_DestroyActor`))

(event `self.ReceiveTick`
  (params (DeltaSeconds :type "Float (single-precision)"))
  (`self.K2_SetActorLocation` (+ (`SceneComponent.K2_GetComponentLocation` (`self.DefaultSceneRoot`)) (* DeltaSeconds (* (`self.MoveVector`) (`self.Speed`)))) true))

(fn `UserConstructionScript`)