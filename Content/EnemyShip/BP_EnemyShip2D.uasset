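; Enemy ship for a 2D shooter that fires projectiles and explodes when its HP runs out.
; BeginPlay uses CombatStyle to pick a self-repeating delay loop: continuous fire or three-round bursts, both spawning BP_Projectile offset from the hull.
; Continuous fire pauses while over 300 projectiles exist and ends when AbleToShoot is false.
; A Teleport function snaps the root to a target position.
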(event `self.ReceiveBeginPlay`
  (switch `/Game/EnemyShip/ENUM_CombatStyles` (`self.CombatStyle`)
    (:`NewEnumerator1`
      (`self.ShootContinuous`))
    (:`NewEnumerator2`
      (`self.ShootThreeRoundBurst`))))

(event `Spawn Projectile`
  ;[0 0.01667 0.1] Spawns the projectile - called by shoot loops
  (bind _returnvalue (`|SpawnActorFromClass` "/Game/EnemyShip/BP_Projectile.BP_Projectile_C" (`KismetMathLibrary.MakeTransform` (- (`SceneComponent.K2_GetComponentLocation` (`self.Hull_Parent`)) (`self.ProjectileSpawnOffset`)) (struct) (* (1.0 1.0 1.0) (`self.ProjectileScale`))) "AdjustIfPossibleButAlwaysSpawn" "OverrideRootScale" null self))
  (set `/Game/EnemyShip/BP_Projectile.ProjectileType` "NewEnumerator0" _returnvalue))

(event `self.ReceiveAnyDamage`
  (params (Damage :type "Float (single-precision)") (DamageType :type "DamageType Object Reference") (InstigatedBy :type "Controller Object Reference") (DamageCauser :type "Actor Object Reference"))
  ;[0.1 0.1 0.1] HP a umírání
  (`|ExecutionSequence`
    (:`then_0`
      (set `self.HP` (- (`self.HP`) Damage)))
    (:`then_1`
      (if (<= (`self.HP`) 0.0)
        (`GameplayStatics.SpawnEmitterAtLocation` "/Game/Assets/VFX_Pack/Particles/Explosion/P_Explosion_Big_B.P_Explosion_Big_B" (.location (`SceneComponent.K2_GetComponentToWorld` (`self.Hull_Parent`))) (.rotation (`SceneComponent.K2_GetComponentToWorld` (`self.Hull_Parent`))))
        (`self.K2_DestroyActor`)))))

(fn `Teleport`
  (params (TargetPosition :type "Vector Structure"))
  (if (!= TargetPosition (`SceneComponent.K2_GetComponentLocation` (`self.DefaultSceneRoot`)) :`ErrorTolerance` 0.01)
    (`SceneComponent.K2_SetWorldLocation` (`self.DefaultSceneRoot`) TargetPosition false true)
    (`KismetSystemLibrary.PrintString` "Teleporting!")))

(fn `UserConstructionScript`)