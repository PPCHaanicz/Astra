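; BP_EnemyShip is an AI enemy ship that takes damage and explodes.
; AnyDamage subtracts from Health, or spawns an explosion at HullParent and destroys the actor when the hit is lethal.
; SetBBPlayerReferences caches the player ship and writes its reference and body location to the Blackboard.
; BeginPlay spawns projectiles at the world origin in an endless loop with no delay, and GetFlyingTarget is an empty stub.
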(event `self.ReceiveAnyDamage`
  (params (Damage :type "Float (single-precision)") (DamageType :type "DamageType Object Reference") (InstigatedBy :type "Controller Object Reference") (DamageCauser :type "Actor Object Reference"))
  (bind _health (`self.Health`))
  (bind _hull_parent (`self.Hull_Parent`))
  ;[0.1 0.1 0.1] Damage a umírání
  (if (>= Damage _health)
    (`GameplayStatics.SpawnEmitterAtLocation` "/Game/Assets/VFX_Pack/Particles/Explosion/P_Explosion_Big_B.P_Explosion_Big_B" (`SceneComponent.K2_GetComponentLocation` _hull_parent) (`SceneComponent.K2_GetComponentRotation` _hull_parent))
    (`self.K2_DestroyActor`)
    (else
      (set `self.Health` (- _health Damage)))))

(event `self.ReceiveBeginPlay`
  (while true
    (`|SpawnActorFromClass` "/Game/EnemyShip/BP_Projectile.BP_Projectile_C" (`KismetMathLibrary.MakeTransform` (0.0 0.0 0.0)) "Undefined" "OverrideRootScale" null null)))

(fn `Get Flying Target`)

(fn `Set BB Player References`
  (params (Object :type "Object Object Reference"))
  (returns (PlayerREF :type "/Game/PlayerShip/BP_PlayerShip Object Reference"))
  (locals (`BB REF Key` :type Name :default "None") (`BB Location Key` :type Name :default "None"))
  (bind _returnvalue (`AIBlueprintHelperLibrary.GetBlackboard` null))
  (bind _asbp_player_ship (cast `/Game/PlayerShip/BP_PlayerShip` Object))
  (bind _output_get (set `self.PlayerREF` _asbp_player_ship))
  (`BlackboardComponent.SetValueAsObject` _returnvalue (`local.BB REF Key`) _output_get)
  (`BlackboardComponent.SetValueAsVector` _returnvalue (`local.BB Location Key`) (`SceneComponent.K2_GetComponentLocation` (`/Game/PlayerShip/BP_PlayerShip.Body` _output_get)))
  (return (`self.PlayerREF`)))

(fn `UserConstructionScript`)