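; BP_EnemySpawner is an enemy spawner actor that creates BP_EnemyShip2D ships at its own location.
; SpawnEnemy passes a CombatStyle to each ship, applies the configured start rotation and uniform scale, and prints a debug message.
; A separate MoveEnemyToField function, not called here, steps a ship's HullParent toward a target with VInterpTo.
; Its while loop runs without yielding, so the whole move completes within one frame.
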(event `SpawnEnemy`
  (params (CombatStyle :type "/Game/EnemyShip/ENUM_CombatStyles Enum" :default "NewEnumerator0"))
  (`|SpawnActorFromClass` "/Game/EnemyShip/BP_EnemyShip2D.BP_EnemyShip2D_C" (`KismetMathLibrary.MakeTransform` (.location (`SceneComponent.K2_GetComponentToWorld` (`self.DefaultSceneRoot`))) (`self.StartRotation`) (* (`self.StartScale`) (1.0 1.0 1.0))) "AlwaysSpawn" "OverrideRootScale" null CombatStyle null)
  (`KismetSystemLibrary.PrintString` "Spawned new ship!"))

(fn `MoveEnemyToField`
  (params (`Target Location` :type "Vector Structure") (ShipReference :type "/Game/EnemyShip/BP_EnemyShip Object Reference"))
  (locals (ShipREF :type "StaticMeshComponent Object Reference") (`Current Location` :type "Vector Structure") (`Target Field Location` :type "Vector Structure"))
  (bind _returnvalue (`KismetMathLibrary.VInterpTo` (`local.Current Location`) (`local.Target Field Location`) (`GameplayStatics.GetWorldDeltaSeconds`) 5.0))
  (set `local.Target Field Location` `Target Location`)
  (bind _output_get (set `local.ShipREF` (`/Game/EnemyShip/BP_EnemyShip.Hull_Parent` ShipReference)))
  (set `local.Current Location` (`SceneComponent.K2_GetComponentLocation` _output_get))
  (while (!= (`local.Current Location`) (`local.Target Field Location`) :`ErrorTolerance` 1.0)
    (`SceneComponent.K2_SetWorldLocation` (`local.ShipREF`) _returnvalue false false)
    (set `local.Current Location` _returnvalue))
  (return))

(fn `UserConstructionScript`)