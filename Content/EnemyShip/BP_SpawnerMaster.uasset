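; Master spawner actor that keeps the enemy population topped up through the level's BP_EnemySpawner actors.
; On BeginPlay it collects all spawners, spawns one enemy from each and tracks the count.
; Tick prints the count and, through a Gate, spawns enemies of a randomly selected enum option at random spawners until the maximum closes it.
; EnemyDied decrements the count and reopens the Gate after a random delay.
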(event `self.ReceiveBeginPlay`
  (bind _outactors (`GameplayStatics.GetAllActorsOfClass` "/Game/EnemyShip/BP_EnemySpawner.BP_EnemySpawner_C"))
  (set `self.Spawners` _outactors)
  (`|ExecutionSequence`
    (:`then_0`
      (for _array_element (`self.Spawners`)
        (`/Game/EnemyShip/BP_EnemySpawner.SpawnEnemy` _array_element "NewEnumerator2")
        (`/Engine/EditorBlueprintResources/StandardMacros.IncrementInt` (`self.EnemyCount`))))))

(event `self.ReceiveTick`
  (params (DeltaSeconds :type "Float (single-precision)"))
  (`KismetSystemLibrary.PrintString` (`KismetStringLibrary.Conv_IntToString` (`self.EnemyCount`)))
  (`/Engine/EditorBlueprintResources/StandardMacros.Gate` false :!label _label
    (:`Exit`
      (if (< (`self.EnemyCount`) (`self.MaximumEnemyCount`))
        (`/Game/EnemyShip/BP_EnemySpawner.SpawnEnemy` (`KismetArrayLibrary.Array_Random` (`self.Spawners`)) (select `int` (`KismetMathLibrary.RandomIntegerInRange` 0 2) :`0` "NewEnumerator1" :`1` "NewEnumerator2" :`2` "NewEnumerator2" :!type "/Game/EnemyShip/ENUM_CombatStyles Enum"))
        (bind _result (`/Engine/EditorBlueprintResources/StandardMacros.IncrementInt` (`self.EnemyCount`))
          (:`  `
            (if (>= _result (`self.MaximumEnemyCount`))
              (goto _label :!via `Close`))))))))

(event `EnemyDied`
  (`/Engine/EditorBlueprintResources/StandardMacros.DecrementInt` (`self.EnemyCount`)
    (:`  `
      (`KismetSystemLibrary.Delay` (`KismetMathLibrary.RandomFloatInRange` 2.0 5.0))
      (goto _label :!via `Open`))))

(fn `UserConstructionScript`)