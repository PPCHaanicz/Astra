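; Player ship with physics-driven flight and hitscan lasers that damage BP_EnemyShip actors.
; Eased thrust input sets a forward velocity applied each tick, Brake toggles it to zero, torque handles pitch, yaw and roll, and Boost is disabled.
; Shots alternate between socket pairs, converging ahead of the hull, with a cooldown and Niagara beams.
; Timed Overdrive fires all four weapons using separate damage and debug traces, without beams.
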(event `self.ReceiveBeginPlay`
  (set `self.Thrust` (/ (`self.MaxThrust`) 2.0)))

(event `InputAction|Shoot`
  (params (Key :type "Key Structure"))
  (bind _hull (`self.Hull`))
  (bind _returnvalue (+ (* (`KismetMathLibrary.GetUpVector` (`SceneComponent.K2_GetComponentRotation` (`self.Hull`))) (`self.WeaponsRange`)) (`SceneComponent.K2_GetComponentLocation` (`self.Hull`))))
  ;[0.1979 0.1979 0.1979] Střelba
  (:`Pressed`
    (if (`self.CanShoot`)
      (switch `/Game/Assets/PlayerShip/ENUM_WeaponStates` (`self.Alternation`) ; Věc co způsobí že se střídá levá a pravá strana
        (:`NewEnumerator1`
          (`|ExecutionSequence`
            (:`then_0`
              (`self.Shoot` "NewEnumerator2" (`SceneComponent.GetSocketLocation` (`self.Hull`) "Weapon1") (`SceneComponent.GetSocketLocation` (`self.Hull`) "Weapon3") _returnvalue))
            (:`then_1`
              (set `self.CanShoot` false)
              (`KismetSystemLibrary.Delay` (`self.WeaponsCD`))
              (set `self.CanShoot` true))))
        (:`NewEnumerator2`
          (`|ExecutionSequence`
            (:`then_0`
              (`self.Shoot` "NewEnumerator1" (`SceneComponent.GetSocketLocation` (`self.Hull`) "Weapon2") (`SceneComponent.GetSocketLocation` (`self.Hull`) "Weapon4") _returnvalue))
            (:`then_1`
              (set `self.CanShoot` false)
              (`KismetSystemLibrary.Delay` (`self.WeaponsCD`))
              (set `self.CanShoot` true))))
        (:`NewEnumerator3`
          (`|ExecutionSequence`
            (:`then_0`
              (`self.ShootOverdrive` (`SceneComponent.GetSocketLocation` _hull "Weapon1") (`SceneComponent.GetSocketLocation` _hull "Weapon3") (`SceneComponent.GetSocketLocation` _hull "Weapon2") (`SceneComponent.GetSocketLocation` _hull "Weapon4") _returnvalue))
            (:`then_1`
              (set `self.CanShoot` false)
              (`KismetSystemLibrary.Delay` (`self.WeaponsCD`))
              (set `self.CanShoot` true))))))))

(event `InputAction|Overdrive`
  (params (Key :type "Key Structure"))
  ;[0.1979 0.1979 0.1979] Střelba
  ;;[0.2812 0.2812 0.2812] pewpew dělají větší brrrrrrrrr
  (:`Pressed`
    (set `self.Alternation` "NewEnumerator3")
    (set `self.Overdrive` true)
    (`KismetSystemLibrary.Delay` 15.0)
    (set `self.Alternation` "NewEnumerator1")
    (set `self.Overdrive` false)))

(event `InputAxis|Thrust`
  (params (AxisValue :type "Float (single-precision)"))
  ;[0.1458 0.1458 0.1458] Forward Speed handling
  (`|ExecutionSequence`
    (:`then_0`
      (if (`self.Boost`)
        ;;[0.1302 0.1302 0.1302] Boost, used when Boost == True, momentálně unused
        (if (not (`KismetMathLibrary.NearlyEqual_FloatFloat` AxisValue 0.0 0.1))
          (set `self.Thrust` (`KismetMathLibrary.FInterpTo` (`self.Thrust`) (`KismetMathLibrary.Lerp` 0.0 (`self.MaxThrust`) (/ (+ 0.0 AxisValue) (`self.BoostSpeedCoef`))) (`GameplayStatics.GetWorldDeltaSeconds`) (`self.SpeedGain`))))
        (elif (not (`KismetMathLibrary.NearlyEqual_FloatFloat` AxisValue 0.0 0.1))
          (set `self.Thrust` (`KismetMathLibrary.FInterpTo` (`self.Thrust`) (`KismetMathLibrary.Lerp` 50.0 (`self.MaxThrust`) (/ (+ AxisValue 1.0) 2.0)) (`GameplayStatics.GetWorldDeltaSeconds`) (`self.SpeedGain`))) ; Thrust gets calculated through lerp magic
        )))
    (:`then_1`
      (if (not (`self.Brake`))
        (set `self.ForwardVelocity` (* (`SceneComponent.GetUpVector` (`self.Body`)) (`self.Thrust`))) ; Here we set the actual vector
        (else
          (set `self.ForwardVelocity` (0.0 0.0 0.0)))))))

(event `InputAction|Boost`
  (params (Key :type "Key Structure"))
  ;[0.1458 0.1458 0.1458] Forward Speed handling
  (:`Pressed`
    (set `self.Boost` false) ; Tady True aby se zapnul Boost
  )
  (:`Released`
    (set `self.Boost` false)))

(event `InputAction|Brake`
  (params (Key :type "Key Structure"))
  ;[0.1458 0.1458 0.1458] Forward Speed handling
  (:`Pressed`
    (set `self.Brake` (not (`self.Brake`)))))

(event `self.ReceiveTick`
  (params (DeltaSeconds :type "Float (single-precision)"))
  ;[0.1458 0.1458 0.1458] Forward Speed handling
  (`PrimitiveComponent.SetPhysicsLinearVelocity` (`self.Body`) (* (`self.ForwardVelocity`) (`self.VelocityMultiplier`)) false "None"))

(event `InputAxis|MoveUp`
  (params (AxisValue :type "Float (single-precision)"))
  ;[0.0625 0.0625 0.0625] 3 degrees of freedom dělají brrrrrrrr - vectory nesouhlasej ale oh well
  (`PrimitiveComponent.AddTorqueInDegrees` (`self.Body`) (* (`SceneComponent.GetForwardVector` (`self.Body`)) (* AxisValue (`self.ForwardTorquePower`))) "None" true))

(event `InputAxis|MoveRight`
  (params (AxisValue :type "Float (single-precision)"))
  ;[0.0625 0.0625 0.0625] 3 degrees of freedom dělají brrrrrrrr - vectory nesouhlasej ale oh well
  (`PrimitiveComponent.AddTorqueInDegrees` (`self.Body`) (* (`SceneComponent.GetRightVector` (`self.Body`)) (* AxisValue (`self.SideTorquePower`))) "None" true))

(event `InputAxis|Roll`
  (params (AxisValue :type "Float (single-precision)"))
  ;[0.0625 0.0625 0.0625] 3 degrees of freedom dělají brrrrrrrr - vectory nesouhlasej ale oh well
  (`PrimitiveComponent.AddTorqueInDegrees` (`self.Body`) (* (`SceneComponent.GetUpVector` (`self.Body`)) (* AxisValue (`self.RotationTorque`))) "None" true))

(fn `SpawnLaserBeam`
  (params (BeamStart :type "Vector Structure") (BeamEnd :type "Vector Structure") (isHit :type Boolean) (OutHit :type "HitResult Structure"))
  (locals (TraceStart :type "Vector Structure") (TraceEnd :type "Vector Structure") (NSRef :type "NiagaraComponent Object Reference"))
  (`|ExecutionSequence`
    (:`then_0`
      (set `local.TraceStart` BeamStart)
      (set `local.TraceEnd` BeamEnd)
      (bind _returnvalue (`NiagaraFunctionLibrary.SpawnSystemAtLocation` "/Game/Framework/NiagaraFX/NS_LaserBeam.NS_LaserBeam" (`self.K2_GetActorLocation`)))
      (bind _output_get (set `local.NSRef` _returnvalue))
      (`FXSystemComponent.SetVectorParameter` _output_get "BeamStart" (`local.TraceStart`)))
    (:`then_1`
      (if isHit
        (`FXSystemComponent.SetVectorParameter` (`local.NSRef`) "BeamEnd" (`.ImpactPoint` (`GameplayStatics.BreakHitResult` OutHit)))
        (else
          (`FXSystemComponent.SetVectorParameter` (`local.NSRef`) "BeamEnd" (`local.TraceEnd`)))))))

(fn `UserConstructionScript`)