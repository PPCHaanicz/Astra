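; Skybox actor that applies a configurable material to its static mesh and controls the sky's look.
; Its construction script writes size, brightness, star brightness, scene brightness and power to the PC_Skybox Material Parameter Collection.
; BeginPlay caches the actor's rotation, but the incremental spin logic is disconnected from Tick, noted as broken because the mesh rotates while the material stays the same.
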(event `self.ReceiveBeginPlay`
  (set `self.CurrentRot` (`self.K2_GetActorRotation` self)))

(event `self.ReceiveTick`
  (params (DeltaSeconds :type "Float (single-precision)"))
  ;[0.1 0.1 0.1] Rotation thing - doesn't work | the SM rotates but the mat stays the same
)

(fn `UserConstructionScript`
  (`PrimitiveComponent.SetMaterial` (`self.StaticMesh`) 0 (`self.Material`))
  (`KismetMaterialLibrary.SetScalarParameterValue` "/Game/Assets/Skybox/PC_Skybox.PC_Skybox" "Size" (`self.Size (Mat 2)`))
  (`KismetMaterialLibrary.SetScalarParameterValue` "/Game/Assets/Skybox/PC_Skybox.PC_Skybox" "Brightness" (`self.Brightness (Mat 2)`))
  (`KismetMaterialLibrary.SetScalarParameterValue` "/Game/Assets/Skybox/PC_Skybox.PC_Skybox" "Star Brightness" (`self.Star Brightness`))
  (`KismetMaterialLibrary.SetScalarParameterValue` "/Game/Assets/Skybox/PC_Skybox.PC_Skybox" "Scene Brightness" (`self.Scene Brightness`))
  (`KismetMaterialLibrary.SetScalarParameterValue` "/Game/Assets/Skybox/PC_Skybox.PC_Skybox" "Power" (`self.Power`)))