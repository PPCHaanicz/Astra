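; Main game mode that tracks difficulty, survival score and player death, with an unfinished objective chain.
; BeginPlay loads difficulty from a save slot, and Tick adds capped time-based score while the player lives, printing difficulty for debug.
; PlayerDied appends the score to an existing save's list, re-saves it sorted ascending, and pauses the game.
; Objective step functions and completion check are stubs, and death-screen and HUD calls are disconnected.
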(event `self.ReceiveBeginPlay`
  (set `self.PlayerAlive` true)
  (bind _returnvalue (`GameplayStatics.LoadGameFromSlot` "Diff"))
  (set `self.Difficulty` (`/Game/Framework/BP_SaveDiff.Difficulty` (cast `/Game/Framework/BP_SaveDiff` _returnvalue :!pure true))))

(event `ChangeDifficulty`
  (params (Selection :type String))
  (switch `string` Selection
    (:`Easy`
      (set `self.Difficulty` "NewEnumerator0"))
    (:`Normal`
      (set `self.Difficulty` "NewEnumerator1"))
    (:`Hard`
      (set `self.Difficulty` "NewEnumerator2"))
    (:`Nightmare`
      (set `self.Difficulty` "NewEnumerator3"))))

(event `self.ReceiveTick`
  (params (DeltaSeconds :type "Float (single-precision)"))
  (if (`self.PlayerAlive`)
    (`self.AddScore` (* DeltaSeconds (`self.BaseScorePerSecond`)))
    (`KismetSystemLibrary.PrintString` (`|GetEnumeratorNameAsString` (`self.Difficulty`)) true true (struct :`G` 0.66 :`B` 1.0 :`A` 1.0) 0.0)))

(event `AddScore`
  (params (Amount :type "Float (double-precision)"))
  (bind _returnvalue (+ Amount (`self.PlayerScore`)))
  (if (< _returnvalue 99999.0)
    (set `self.PlayerScore` _returnvalue)
    (else
      (set `self.PlayerScore` 99999.0))))

(event `PlayerDied`
  (`KismetSystemLibrary.PrintString` "gmmain event received" true true (struct :`G` 0.66 :`B` 1.0 :`A` 1.0) 5.0)
  (`|ExecutionSequence`
    (:`then_0`
      (set `self.PlayerAlive` false)
      (`KismetSystemLibrary.PrintString` "player unalived" true true (struct :`G` 0.66 :`B` 1.0 :`A` 1.0) 5.0))
    (:`then_1`
      (bind _returnvalue (`GameplayStatics.LoadGameFromSlot` "Score"))
      (bind _asbp_save_score (cast `/Game/Framework/BP_SaveScore` _returnvalue)
        (:`then`
          (`KismetSystemLibrary.PrintString` "cast savescore succesful" true true (struct :`G` 0.66 :`B` 1.0 :`A` 1.0) 5.0)
          (bind _playerscorelist (`/Game/Framework/BP_SaveScore.PlayerScoreList` _asbp_save_score))
          (`KismetArrayLibrary.Array_Append` _playerscorelist (`|MakeArray` (`self.PlayerScore`)))
          (bind _returnvalue_2 (`GameplayStatics.CreateSaveGameObject` "/Game/Framework/BP_SaveScore.BP_SaveScore_C"))
          (set `/Game/Framework/BP_SaveScore.PlayerScoreList` (`LowEntryExtendedStandardLibrary.SortFloatArray` _playerscorelist) _returnvalue_2)
          (bind _returnvalue_3 (`GameplayStatics.SaveGameToSlot` _returnvalue_2 "Score"))
          (if _returnvalue_3
            (`KismetSystemLibrary.PrintString` "save succeeded" true true (struct :`G` 0.66 :`B` 1.0 :`A` 1.0) 5.0)
            (else
              (`KismetSystemLibrary.PrintString` "save failed" true true (struct :`G` 0.66 :`B` 1.0 :`A` 1.0) 5.0))))
        (:`CastFailed`
          (`KismetSystemLibrary.PrintString` "cast savescore failed" true true (struct :`G` 0.66 :`B` 1.0 :`A` 1.0) 5.0))))
    (:`then_3`
      (`GameplayStatics.SetGamePaused` true)
      (`KismetSystemLibrary.PrintString` "game paused"))))

(fn `EnemyDestroyed`)

(fn `IsObjectiveComplete`
  (params (`Current Objective` :type "/Game/Framework/ENUM_Objectives Enum" :default "NewEnumerator0"))
  (returns (IsComplete :type Boolean))
  (switch `/Game/Framework/ENUM_Objectives` `Current Objective`))

(fn `NewDestroyEnemy`)

(fn `NewFlyToLocation`)

(fn `NewObjective`
  (params (CurrentObjective :type "/Game/Framework/ENUM_Objectives Enum" :default "NewEnumerator0"))
  (switch `/Game/Framework/ENUM_Objectives` CurrentObjective
    (:`NewEnumerator0`
      (`self.NewFlyToLocation`)
      (set `self.Objective` "NewEnumerator1"))
    (:`NewEnumerator1`
      (`self.NewDestroyEnemy`)
      (set `self.Objective` "NewEnumerator2"))
    (:`NewEnumerator2`
      (`self.Victory`)
      (set `self.Objective` "NewEnumerator3"))))

(fn `UserConstructionScript`)

(fn `Victory`)