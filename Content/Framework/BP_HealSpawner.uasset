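; BP_HealSpawner is a spawner actor that periodically creates BP_HealPickup actors at its own location, scaled by ProjectileScale.
; BeginPlay waits a random delay, then loops: spawn, wait a fixed interval, then count all heal pickups in the world.
; While the count exceeds a small cap it polls again after a short delay.
; Otherwise it spawns again if AbleToSpawn is true; if false, the loop ends.
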(event `Spawn Heal`
  ;[0.1 0.1 0.1] Spawns the projectile - ctrl c from EnemyShip
  (`|SpawnActorFromClass` "/Game/Framework/BP_HealPickup.BP_HealPickup_C" (`KismetMathLibrary.MakeTransform` (`SceneComponent.K2_GetComponentLocation` (`self.DefaultSceneRoot`)) (struct) (* (1.0 1.0 1.0) (`self.ProjectileScale`))) "AdjustIfPossibleButAlwaysSpawn" "OverrideRootScale" null self)
  (`KismetSystemLibrary.PrintString` "Spawned Heal"))

(event `self.ReceiveBeginPlay`
  (`KismetSystemLibrary.Delay` (`KismetMathLibrary.RandomFloatInRange` 2.0 30.0))
  (`self.Spawn Heal` :!label _label)
  (`KismetSystemLibrary.Delay` 25.0)
  (bind _outactors (`GameplayStatics.GetAllActorsOfClass` "/Game/Framework/BP_HealPickup.BP_HealPickup_C" :!label _label_2))
  (if (<= (`KismetArrayLibrary.Array_Length` _outactors) 5)
    (if (`self.AbleToSpawn`)
      (goto _label))
    (else
      (`KismetSystemLibrary.Delay` 2.0)
      (goto _label_2))))

(fn `UserConstructionScript`)