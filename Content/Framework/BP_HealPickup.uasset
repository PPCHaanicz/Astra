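; BP_HealPickup is a moving health pickup that heals the 2D player ship on contact.
; It attaches a Niagara heal effect to its collision sphere and moves each tick along a move vector at a set speed, using sweep.
; Overlap with BP_PlayerShip2D calls the ship's heal event with its regen amount and destroys the pickup, which otherwise destroys itself after a short lifetime.
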(event `self.ReceiveBeginPlay`
  (`NiagaraFunctionLibrary.SpawnSystemAttached` "/Game/Assets/EnergyBall/NS_EnergyBall_Heal.NS_EnergyBall_Heal" (`self.CollisionSphere`) "None" (0.0 0.0 0.0) (struct :`Yaw` 90.0) "KeepRelativeOffset")
  (`KismetSystemLibrary.Delay` 5.5)
  (`self.K2_DestroyActor`))

(event `self.ReceiveTick`
  (params (DeltaSeconds :type "Float (single-precision)"))
  (`self.K2_SetActorLocation` (+ (`SceneComponent.K2_GetComponentLocation` (`self.DefaultSceneRoot`)) (* DeltaSeconds (* (`self.MoveVector`) (`self.Speed`)))) true))

(event `self.CollisionSphere.OnComponentBeginOverlap`
  (params (OverlappedComponent :type "PrimitiveComponent Object Reference") (OtherActor :type "Actor Object Reference") (OtherComp :type "PrimitiveComponent Object Reference") (OtherBodyIndex :type Integer) (bFromSweep :type Boolean) (SweepResult :type "HitResult Structure (by ref)"))
  (bind _asbp_player_ship_2d (cast `/Game/PlayerShip/BP_PlayerShip2D` OtherActor))
  (`/Game/PlayerShip/BP_PlayerShip2D.Event Heal` _asbp_player_ship_2d (`self.HealthRegen`))
  (`self.K2_DestroyActor`))

(fn `UserConstructionScript`)