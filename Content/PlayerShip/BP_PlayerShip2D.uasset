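; Player ship pawn for a 2D shooter, with movement input gated by fixed X/Y bounds.
; Shooting alternates socket pairs on a cooldown, while a timed Overdrive fires all four using separate damage, with line traces damaging enemy ships and driving Niagara laser beams.
; Projectile overlaps reduce health and spawn explosions, but the death check is disconnected.
; The ShowObjective input just adds a large fixed score through GM_Main.
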(event `InputAction|Shoot`
  (params (Key :type "Key Structure"))
  (bind _hull (`self.Hull`))
  (bind _hull_2 (`self.Hull`))
  (bind _hull_3 (`self.Hull`))
  ;[0.1 0.1 0.1] Střelba
  (:`Pressed`
    (if (`self.CanShoot`)
      (switch `/Game/PlayerShip/ENUM_WeaponStates` (`self.Alternation`) ; Věc co způsobí že se střídá levá a pravá strana
        (:`NewEnumerator1`
          (`|ExecutionSequence`
            (:`then_0`
              (`self.Shoot` (`SceneComponent.GetSocketLocation` _hull_3 "Weapon1") (`SceneComponent.GetSocketLocation` _hull_3 "Weapon3") "NewEnumerator2"))
            (:`then_1`
              (set `self.CanShoot` false)
              (`KismetSystemLibrary.Delay` (`self.WeaponsCD`))
              (set `self.CanShoot` true))))
        (:`NewEnumerator2`
          (`|ExecutionSequence`
            (:`then_0`
              (`self.Shoot` (`SceneComponent.GetSocketLocation` _hull_2 "Weapon2") (`SceneComponent.GetSocketLocation` _hull_2 "Weapon4") "NewEnumerator1"))
            (:`then_1`
              (set `self.CanShoot` false)
              (`KismetSystemLibrary.Delay` (`self.WeaponsCD`))
              (set `self.CanShoot` true))))
        (:`NewEnumerator3`
          (`|ExecutionSequence`
            (:`then_0`
              (`self.ShootOverdrive` (`SceneComponent.GetSocketLocation` _hull "Weapon1") (`SceneComponent.GetSocketLocation` _hull "Weapon3") (`SceneComponent.GetSocketLocation` _hull "Weapon2") (`SceneComponent.GetSocketLocation` _hull "Weapon4")))
            (:`then_1`
              (set `self.CanShoot` false)
              (`KismetSystemLibrary.Delay` (`self.WeaponsCD`))
              (set `self.CanShoot` true))))))))

(event `InputAction|Overdrive`
  (params (Key :type "Key Structure"))
  ;[0.1 0.1 0.1] Střelba
  ;;[0.1 0.1 0.1] pewpew dělají větší brrrrrrrrr
  (:`Pressed`
    (set `self.Alternation` "NewEnumerator3")
    (set `self.Overdrive` true)
    (`KismetSystemLibrary.Delay` 15.0)
    (set `self.Alternation` "NewEnumerator1")
    (set `self.Overdrive` false)))

(event `self.ReceiveBeginPlay`
  (set `self.Health` (`self.MaxHealth`))
  (set `self.GamemodeREF` (cast `/Game/Framework/GM_Main` (`GameplayStatics.GetGameMode`) :!pure true)))

(event `self.ReceiveTick`
  (params (DeltaSeconds :type "Float (single-precision)")))

(event `InputAxis|MoveForward`
  (params (AxisValue :type "Float (single-precision)"))
  (`self.MoveForward` AxisValue))

(event `InputAxis|MoveSideways`
  (params (AxisValue :type "Float (single-precision)"))
  (`self.MoveSideways` AxisValue))

(event `self.HitBox.OnComponentBeginOverlap`
  (params (OverlappedComponent :type "PrimitiveComponent Object Reference") (OtherActor :type "Actor Object Reference") (OtherComp :type "PrimitiveComponent Object Reference") (OtherBodyIndex :type Integer) (bFromSweep :type Boolean) (SweepResult :type "HitResult Structure (by ref)"))
  (bind _asbp_projectile (cast `/Game/EnemyShip/BP_Projectile` OtherActor))
  (set `self.ProjectileREF` _asbp_projectile)
  (bind _output_get (set `self.Health` (- (`self.Health`) 10.0)))
  (`|ExecutionSequence`
    (:`then_0`
      (`GameplayStatics.SpawnEmitterAtLocation` "/Game/Assets/VFX_Pack/Particles/Explosion/P_Explosion_Big_B.P_Explosion_Big_B" (`SceneComponent.K2_GetComponentLocation` (`/Game/EnemyShip/BP_Projectile.Sphere` (`self.ProjectileREF`))) (struct) (* (1.0 1.0 1.0) 0.3))
      (`self.K2_DestroyActor` (`self.ProjectileREF`)))))

(event `InputAction|ShowObjective`
  (params (Key :type "Key Structure"))
  (:`Pressed`
    (`/Game/Framework/GM_Main.AddScore` (`self.GamemodeREF`) 151561.0)))

(fn `HitReg`
  (params (`Weapon Socket` :type "Vector Structure") (End :type "Vector Structure"))
  (returns (TraceStart :type "Vector Structure") (TraceEnd :type "Vector Structure") (isHit :type Boolean) (outHit :type "HitResult Structure"))
  (bind (_outhit _returnvalue) (`KismetSystemLibrary.LineTraceSingle` :`Start` `Weapon Socket` :`End` End :`TraceChannel` "TraceTypeQuery3" :`bTraceComplex` true :`DrawTime` 15.0))
  (bind _asbp_enemy_ship_2d (cast `/Game/EnemyShip/BP_EnemyShip2D` (`.HitActor` (`GameplayStatics.BreakHitResult` _outhit)))
    (:`then`
      (`GameplayStatics.ApplyDamage` _asbp_enemy_ship_2d (`self.Damage`)))
    (:`CastFailed`
      _))
  (return `Weapon Socket` End _returnvalue _outhit))

(fn `HitReg_Overdrive`
  (params (Start :type "Vector Structure") (End :type "Vector Structure"))
  (returns (TraceStart :type "Vector Structure") (TraceEnd :type "Vector Structure") (isHit :type Boolean) (outHit :type "HitResult Structure"))
  (bind (_outhit _returnvalue) (`KismetSystemLibrary.LineTraceSingle` :`Start` Start :`End` End :`TraceChannel` "TraceTypeQuery3" :`bTraceComplex` true :`DrawTime` 15.0))
  (bind _asbp_enemy_ship_2d (cast `/Game/EnemyShip/BP_EnemyShip2D` (`.HitActor` (`GameplayStatics.BreakHitResult` _outhit)))
    (:`then`
      (`GameplayStatics.ApplyDamage` _asbp_enemy_ship_2d (`self.OverdriveDamage`)))
    (:`CastFailed`
      _))
  (return Start End _returnvalue _outhit))

(fn `MoveForward`
  (params (ScaleValue :type "Float (single-precision)"))
  (locals (AxisScale :type "Float (single-precision)"))
  (bind (_x _y) (`KismetMathLibrary.BreakVector3f` (`SceneComponent.K2_GetComponentLocation` (`self.Body`))))
  (bind _output_get (set `local.AxisScale` ScaleValue))
  (if (> _output_get 0.0)
    (if (< _y 0.0)
      (`self.AddMovementInput` (`KismetMathLibrary.GetForwardVector` (`self.GetControlRotation`)) (`local.AxisScale`) :!label _label)
      (return))
    (elif (> _y -500.0)
      (goto _label))))

(fn `MoveSideways`
  (params (ScaleValue :type "Float (single-precision)"))
  (locals (AxisScale :type "Float (single-precision)"))
  (bind _x (`KismetMathLibrary.BreakVector3f` (`SceneComponent.K2_GetComponentLocation` (`self.Body`))))
  (bind _output_get (set `local.AxisScale` ScaleValue))
  (if (> _output_get 0.0)
    (if (> _x -1000.0)
      (`self.AddMovementInput` (`KismetMathLibrary.GetRightVector` (`self.GetControlRotation`)) (`local.AxisScale`) :!label _label)
      (return))
    (elif (< _x 1000.0)
      (goto _label))))

(fn `SpawnLaserBeam`
  (params (BeamStart :type "Vector Structure") (BeamEnd :type "Vector Structure") (isHit :type Boolean) (OutHit :type "HitResult Structure"))
  (locals (TraceStart :type "Vector Structure") (TraceEnd :type "Vector Structure") (NSRef :type "NiagaraComponent Object Reference"))
  (bind (_bblockinghit _binitialoverlap _time _distance _location _impactpoint) (`GameplayStatics.BreakHitResult` OutHit))
  (`|ExecutionSequence`
    (:`then_0`
      (set `local.TraceStart` BeamStart)
      (set `local.TraceEnd` BeamEnd)
      (bind _returnvalue (`NiagaraFunctionLibrary.SpawnSystemAtLocation` "/Game/Framework/NiagaraFX/NS_LaserBeam.NS_LaserBeam" (`self.K2_GetActorLocation`)))
      (bind _output_get (set `local.NSRef` _returnvalue))
      (`FXSystemComponent.SetVectorParameter` _output_get "BeamStart" (`local.TraceStart`)))
    (:`then_1`
      (if isHit
        (`FXSystemComponent.SetVectorParameter` (`local.NSRef`) "BeamEnd" _impactpoint)
        (`GameplayStatics.SpawnEmitterAtLocation` "/Game/Assets/VFX_Pack/Particles/Destruction/P_Destruction_Metal.P_Destruction_Metal" _impactpoint)
        (else
          (`FXSystemComponent.SetVectorParameter` (`local.NSRef`) "BeamEnd" (`local.TraceEnd`)))))))

(fn `UserConstructionScript`)